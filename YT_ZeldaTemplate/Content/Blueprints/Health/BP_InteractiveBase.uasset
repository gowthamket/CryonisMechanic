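; BP_InteractiveBase is a base interactive actor that reacts when the player touches it.
; When the player pawn begins overlapping its Sphere component, it plays InteractSound at its location and calls PlayerInteract.
; PlayerInteract is empty here, serving as a hook for child Blueprints to supply specific behavior.
; The actor then destroys itself if DestroyOnTouch is set.
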(event `self.Sphere.OnComponentBeginOverlap`
  (params (OverlappedComponent :type "PrimitiveComponent Object Reference") (OtherActor :type "Actor Object Reference") (OtherComp :type "PrimitiveComponent Object Reference") (OtherBodyIndex :type Integer) (bFromSweep :type Boolean) (SweepResult :type "HitResult Structure (by ref)"))
  (bind _output_get (set `self.OtherActor` OtherActor))
  (if (== _output_get (`GameplayStatics.GetPlayerPawn` 0))
    (`GameplayStatics.PlaySoundAtLocation` (`self.InteractSound`) (`self.K2_GetActorLocation`) (struct) 1.0 1.0 0.0 null null null)
    (`self.PlayerInteract`)
    (if (`self.bDestroyOnTouch`)
      (`self.K2_DestroyActor`))))

(fn `PlayerInteract`)

(fn `UserConstructionScript`)