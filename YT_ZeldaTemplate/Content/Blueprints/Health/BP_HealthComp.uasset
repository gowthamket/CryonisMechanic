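; BP_HealthComp is a health component that drives a heart-container health display for the player.
; On BeginPlay it creates WBP_Health, adds it to the viewport and initialises it with the component's heart settings.
; Its add-heart, damage and heal calls forward to that widget.
; When the widget's damage result is false, it stops player 0's Character movement and plays a hit-react montage, so it assumes a Character pawn.
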(event `self.ReceiveBeginPlay`
  (bind _returnvalue (`|CreateWidget` "/Game/Blueprints/UI/WBP_Health.WBP_Health_C"))
  (bind _output_get (set `self.HealthWidgetRef` _returnvalue))
  (`UserWidget.AddToViewport` _output_get 0)
  (`self.InitialiseHealth`))

(fn `AddHeartCall`
  (returns (Return :type Boolean))
  (`/Game/Blueprints/UI/WBP_Health.AddHeart` (`self.HealthWidgetRef`) (`self.bFillHeartOnHeartContainer`) (`self.MaxHeartPerRow`))
  (return false))

(fn `DamageCall`
  (params (Damage :type Integer))
  (returns (Return :type Boolean))
  (bind _returnvalue (`GameplayStatics.GetPlayerCharacter` 0))
  (bind _bdied (`/Game/Blueprints/UI/WBP_Health.TakeDamage` (`self.HealthWidgetRef`) Damage (`self.MaxHeartHealth`)))
  ;[1 1 1] Check if we've just died
  (if (not _bdied)
    ;[1 1 1] Stop Player and call a quick hit montage. NOTE *** Remove this is you're not using the "Character" Class as we're looking for the "MovementComponent" here.
    (`MovementComponent.StopMovementImmediately` (`Character.CharacterMovement` _returnvalue))
    (`Character.PlayAnimMontage` _returnvalue "/Game/Assets/Animations/HitReact_Front_Montage.HitReact_Front_Montage" 1.0 "DefaultSlot")
    (return false)))

(fn `HealCall`
  (params (HealAmount :type Integer))
  (returns (Return :type Boolean))
  (`/Game/Blueprints/UI/WBP_Health.Heal` (`self.HealthWidgetRef`) HealAmount (`self.MaxHeartHealth`))
  (return false))

(fn `InitialiseHealth`
  (`/Game/Blueprints/UI/WBP_Health.InitialiseHealth` (`self.HealthWidgetRef`) (`self.DefaultHeartCount`) (`self.MaxHeartHealth`) (`self.MaxHeartPerRow`)))