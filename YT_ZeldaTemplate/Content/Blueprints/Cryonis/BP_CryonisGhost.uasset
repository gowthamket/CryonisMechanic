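; BP_CryonisGhost is a placement ghost for the Cryonis ability that shows where a spawn can happen.
; On BeginPlay, the AnimateCryo timeline grows the actor's Z scale from zero to TargetZScale, keeping X and Y at one.
; Any overlap with the Box sets SpawnBlocked and hides the mesh, and any end overlap clears the flag and shows it again, without counting remaining overlaps.
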(event `self.ReceiveBeginPlay`
  (`self.AnimateCube`))

(event `AnimateCube`
  (bind (_direction _zscale) (`Timeline|AnimateCryo` :!via `PlayFromStart`)
    (:`Update`
      (`self.SetActorScale3D` (`KismetMathLibrary.MakeVector` 1.0 1.0 (`KismetMathLibrary.Lerp` 0.0 (`self.TargetZScale`) _zscale))))))

(event `self.Box.OnComponentBeginOverlap`
  (params (OverlappedComponent :type "PrimitiveComponent Object Reference") (OtherActor :type "Actor Object Reference") (OtherComp :type "PrimitiveComponent Object Reference") (OtherBodyIndex :type Integer) (bFromSweep :type Boolean) (SweepResult :type "HitResult Structure (by ref)"))
  (set `self.bSpawnBlocked` true)
  (`SceneComponent.SetHiddenInGame` (`self.StaticMesh`) true false))

(event `self.Box.OnComponentEndOverlap`
  (params (OverlappedComponent :type "PrimitiveComponent Object Reference") (OtherActor :type "Actor Object Reference") (OtherComp :type "PrimitiveComponent Object Reference") (OtherBodyIndex :type Integer))
  (set `self.bSpawnBlocked` false)
  (`SceneComponent.SetHiddenInGame` (`self.StaticMesh`) false false))

(fn `UserConstructionScript`)