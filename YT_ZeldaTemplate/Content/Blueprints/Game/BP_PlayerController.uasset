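; Player controller that opens and closes a rune selection menu.
; The RuneSelect input action toggles the menu based on whether a widget reference is valid.
; Opening creates WBP_RuneMenu with a reference back to the controller, adds it to the viewport, shows the cursor and switches to game-and-UI input.
; Closing removes the widget, clears the reference, hides the cursor and restores game-only input.
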(event `InputAction|RuneSelect`
  (params (Key :type "Key Structure"))
  (:`Pressed`
    (`/Engine/EditorBlueprintResources/StandardMacros.IsValid` (`self.RuneWidgetRef`)
      (:`Is Valid`
        (`self.RemoveRuneWidget`))
      (:`Is Not Valid`
        (`self.CreateRuneWidget`)))))

(fn `CreateRuneWidget`
  (bind _returnvalue (`|CreateWidget` "/Game/Blueprints/UI/WBP_RuneMenu.WBP_RuneMenu_C" self self))
  (bind _output_get (set `self.RuneWidgetRef` _returnvalue))
  (`UserWidget.AddToViewport` _output_get 0)
  (`WidgetBlueprintLibrary.SetInputMode_GameAndUIEx` self null)
  (set `self.bShowMouseCursor` true))

(fn `RemoveRuneWidget`
  (`Widget.RemoveFromParent` (`self.RuneWidgetRef`))
  (set `self.RuneWidgetRef` null)
  (`WidgetBlueprintLibrary.SetInputMode_GameOnly` self)
  (set `self.bShowMouseCursor` false))

(fn `UserConstructionScript`)